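; Patrolling enemy for a side-scrolling Paper2D game that can be squashed or can defeat the player.
; It walks along X, reverses through a FlipFlop on each Hit, and yaws FBOpo to match velocity.
; Box1 overlap by a PaperCharacter flattens and destroys it.
; Box overlap shrinks the player; this enemy's second counted overlap freezes and hides them, shows the lose widget and spawns BP_Death.
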(event `self.ReceiveTick`
  (params (DeltaSeconds :type "Float (single-precision)"))
  (`self.AddMovementInput` (`self.World Direction`) 0.2)
  (`self.UpdateControlRotation`))

(event `self.Box1.OnComponentBeginOverlap`
  (params (OverlappedComponent :type "PrimitiveComponent Object Reference") (OtherActor :type "Actor Object Reference") (OtherComp :type "PrimitiveComponent Object Reference") (OtherBodyIndex :type Integer) (bFromSweep :type Boolean) (SweepResult :type "HitResult Structure (by ref)"))
  (cast `PaperCharacter` OtherActor)
  (`CharacterMovementComponent.DisableMovement` (`self.CharacterMovement`))
  (`self.SetActorScale3D` (1.0 1.0 0.3))
  (`|ExecutionSequence`
    (:`then_0`
      (`KismetSystemLibrary.Delay` 0.5)
      (`self.K2_DestroyActor`))
    (:`then_1`
      (`GameplayStatics.PlaySound2D` "/Engine/VREditor/Sounds/UI/Object_Snaps_To_Grid.Object_Snaps_To_Grid" 1.0 1.0 0.0 null null))))

(event `self.ReceiveHit`
  (params (MyComp :type "PrimitiveComponent Object Reference") (Other :type "Actor Object Reference") (OtherComp :type "PrimitiveComponent Object Reference") (bSelfMoved :type Boolean) (HitLocation :type "Vector Structure") (HitNormal :type "Vector Structure") (NormalImpulse :type "Vector Structure") (Hit :type "HitResult Structure (by ref)"))
  (`/Engine/EditorBlueprintResources/StandardMacros.FlipFlop`
    (:`A`
      (set `self.World Direction` (-1.0 0.0 0.0)))
    (:`B`
      (set `self.World Direction` (1.0 0.0 0.0)))))

(event `UpdateControlRotation`
  (`/Engine/EditorBlueprintResources/StandardMacros.IsValid` (`self.FB_Opo`)
    (:`Is Valid`
      (`/Engine/EditorBlueprintResources/StandardMacros.CompareFloat` (.x (`MovementComponent.Velocity` (`self.CharacterMovement`)))
        (:`>`
          (`SceneComponent.K2_SetRelativeRotation` (`self.FB_Opo`) (`KismetMathLibrary.MakeRotator` 0.0 0.0 180.0) false false))
        (:`<`
          (`SceneComponent.K2_SetRelativeRotation` (`self.FB_Opo`) (`KismetMathLibrary.MakeRotator` 0.0) false false))))))

(event `self.Box.OnComponentBeginOverlap`
  (params (OverlappedComponent :type "PrimitiveComponent Object Reference") (OtherActor :type "Actor Object Reference") (OtherComp :type "PrimitiveComponent Object Reference") (OtherBodyIndex :type Integer) (bFromSweep :type Boolean) (SweepResult :type "HitResult Structure (by ref)"))
  (bind _asbp_paper_character (cast `/Game/Characters/BP_Paper_Character` OtherActor))
  (`self.SetActorScale3D` _asbp_paper_character (0.5 0.5 0.5))
  (`|ExecutionSequence`
    (:`then_0`
      (`/Engine/EditorBlueprintResources/StandardMacros.DoOnce` false :!label _label
        (:`Completed`
          (`|ExecutionSequence`
            (:`then_0`
              (`KismetSystemLibrary.Delay` 0.5)
              (bind _result (`/Engine/EditorBlueprintResources/StandardMacros.IncrementInt` (`self.ColCount`))
                (:`  `
                  (bind _output_get (set `self.ColCount` _result))
                  (if (== _output_get 2)
                    (`CharacterMovementComponent.DisableMovement` (`Character.CharacterMovement` _asbp_paper_character))
                    (bind _returnvalue (`|CreateWidget` "/Game/Assets/WBPs/WBP_Lose.WBP_Lose_C"))
                    (`UserWidget.AddToViewport` _returnvalue 0)
                    (`GameplayStatics.PlaySound2D` "/Game/Assets/Sounds/dark-wind-19785.dark-wind-19785" 1.0 1.0 0.0 null null)
                    (`|ExecutionSequence`
                      (:`then_0`
                        (`|SpawnActorFromClass` "/Game/Assets/Death/BP_Death.BP_Death_C" (`KismetMathLibrary.Conv_VectorToTransform` (`CharacterMovementComponent.GetLastUpdateLocation` (`Character.CharacterMovement` _asbp_paper_character))) "Undefined" "OverrideRootScale" null null))
                      (:`then_1`
                        (`self.SetActorHiddenInGame` _asbp_paper_character true)))))))
            (:`then_1`
              (goto _label :!via `Reset`))))))
    (:`then_1`
      (`GameplayStatics.PlaySound2D` "/Engine/VREditor/Sounds/UI/Selection_Changes.Selection_Changes" 1.0 1.0 0.0 null null))))

(fn `UserConstructionScript`)