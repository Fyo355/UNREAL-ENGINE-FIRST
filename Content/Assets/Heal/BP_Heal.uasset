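; BP_Heal is a moving heal pickup that restores the player's paper character to normal size on touch.
; On capsule overlap with BP_Paper_Character, it resets the actor scale, destroys itself, zeroes ColCount on the first BP_Enemy found and plays a sound.
; It walks along the X axis each tick, and a FlipFlop on each Hit event alternates its direction.
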(event `self.CapsuleComponent.OnComponentBeginOverlap`
  (params (OverlappedComponent :type "PrimitiveComponent Object Reference") (OtherActor :type "Actor Object Reference") (OtherComp :type "PrimitiveComponent Object Reference") (OtherBodyIndex :type Integer) (bFromSweep :type Boolean) (SweepResult :type "HitResult Structure (by ref)"))
  (bind _asbp_paper_character (cast `/Game/Characters/BP_Paper_Character` OtherActor))
  (`self.SetActorScale3D` _asbp_paper_character (1.0 1.0 1.0))
  (`self.K2_DestroyActor`)
  (`|ExecutionSequence`
    (:`then_0`
      (bind _outactors (`GameplayStatics.GetAllActorsOfClass` "/Game/Assets/Enemy/BP_Enemy.BP_Enemy_C"))
      (set `/Game/Assets/Enemy/BP_Enemy.ColCount` 0 (`|GetArrayItem` _outactors)))
    (:`then_1`
      (`GameplayStatics.PlaySound2D` "/Engine/VREditor/Sounds/UI/Foliage_Placed.Foliage_Placed" 1.0 1.0 0.0 null null))))

(event `self.ReceiveTick`
  (params (DeltaSeconds :type "Float (single-precision)"))
  (`self.AddMovementInput` (`self.World Direction`) 0.2))

(event `self.ReceiveHit`
  (params (MyComp :type "PrimitiveComponent Object Reference") (Other :type "Actor Object Reference") (OtherComp :type "PrimitiveComponent Object Reference") (bSelfMoved :type Boolean) (HitLocation :type "Vector Structure") (HitNormal :type "Vector Structure") (NormalImpulse :type "Vector Structure") (Hit :type "HitResult Structure (by ref)"))
  (`/Engine/EditorBlueprintResources/StandardMacros.FlipFlop`
    (:`A`
      (set `self.World Direction` (-1.0 0.0 0.0)))
    (:`B`
      (set `self.World Direction` (1.0 0.0 0.0)))))

(fn `UserConstructionScript`)