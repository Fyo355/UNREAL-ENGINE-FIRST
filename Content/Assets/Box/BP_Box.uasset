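; BP_Box is a 2D hit block that bumps when a PaperCharacter overlaps it, releases a BP_Coi actor and then disappears.
; The Box overlap raises the root with MoveComponentTo, then spawns BP_Coi at the Arrow's transform.
; A sequence plays a switch sound while the box pauses briefly, lowers back down and destroys itself.
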(event `self.Box.OnComponentBeginOverlap`
  (params (OverlappedComponent :type "PrimitiveComponent Object Reference") (OtherActor :type "Actor Object Reference") (OtherComp :type "PrimitiveComponent Object Reference") (OtherBodyIndex :type Integer) (bFromSweep :type Boolean) (SweepResult :type "HitResult Structure (by ref)"))
  (bind _defaultsceneroot (`self.DefaultSceneRoot`))
  (bind _defaultsceneroot_2 (`self.DefaultSceneRoot`))
  (bind (_returnvalue_location _returnvalue_rotation) (`KismetMathLibrary.BreakTransform` (`SceneComponent.GetRelativeTransform` _defaultsceneroot_2)))
  (bind (_returnvalue_location_2 _returnvalue_rotation_2) (`KismetMathLibrary.BreakTransform` (`SceneComponent.GetRelativeTransform` _defaultsceneroot)))
  (cast `PaperCharacter` OtherActor)
  (`KismetSystemLibrary.MoveComponentTo` _defaultsceneroot (+ _returnvalue_location_2 (0.0 0.0 40.0)) _returnvalue_rotation_2)
  (`|SpawnActorFromClass` "/Game/Assets/Coin/BP_Coi.BP_Coi_C" (`SceneComponent.K2_GetComponentToWorld` (`self.Arrow`)) "Undefined" "OverrideRootScale" null null)
  (`|ExecutionSequence`
    (:`then_0`
      (`KismetSystemLibrary.Delay` 0.2)
      (`KismetSystemLibrary.MoveComponentTo` _defaultsceneroot_2 (+ _returnvalue_location (0.0 0.0 -40.0)) _returnvalue_rotation)
      (`self.K2_DestroyActor`))
    (:`then_1`
      (`GameplayStatics.PlaySound2D` "/Engine/VREditor/Sounds/UI/Flashlight_Switch.Flashlight_Switch" 1.0 1.0 0.0 null null))))

(fn `UserConstructionScript`)